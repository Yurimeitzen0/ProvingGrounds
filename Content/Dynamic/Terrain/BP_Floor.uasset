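; Infinite-terrain floor tile that fills itself with scattered props and AI characters on BeginPlay, behind a wall that starts with a red barrier material.
; When the player enters LockingVolume, the wall turns see-through and non-colliding, the game mode spawns a tile, and the player regains some health.
; On exit, the wall locks again and the game mode removes a tile.
; GetAttachLocation exposes the Arrow's world transform as an attach point.
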(event OnComponentBeginOverlap(LockingVolume)
  (params (OverlappedComponent :type Primitive%20Component%20Object%20Reference) (OtherActor :type Actor%20Object%20Reference) (OtherComp :type Primitive%20Component%20Object%20Reference) (OtherBodyIndex :type Integer) (bFromSweep :type Boolean) (SweepResult :type Hit%20Result%20Structure%20%28by%20ref%29))
  (Utilities|IsPlayerCharacter OtherActor
    (:True
      (CallFunction|Unlock)
      (bind _asbp_infinite_terrain_game_mode (Utilities|Casting|CastToBP_InfiniteTerrainGameMode (Game|GetGameMode)))
      (Default|SpawnTile _asbp_infinite_terrain_game_mode)
      (bind _astp_character (Utilities|Casting|CastToTP_Character OtherActor))
      (Variables|/Game/Dynamic/Character/Blueprints/TP_Character.TP_Character_C|SetHealth _astp_character (Math|Float|Clamp(Float) (+ (Variables|/Game/Dynamic/Character/Blueprints/TP_Character.TP_Character_C|GetHealth _astp_character) 5.0) 0.0 1e+02)))))

(event OnComponentEndOverlap(LockingVolume)
  (params (OverlappedComponent :type Primitive%20Component%20Object%20Reference) (OtherActor :type Actor%20Object%20Reference) (OtherComp :type Primitive%20Component%20Object%20Reference) (OtherBodyIndex :type Integer))
  (Utilities|IsPlayerCharacter OtherActor
    (:True
      (CallFunction|Lock)
      (bind _asbp_infinite_terrain_game_mode (Utilities|Casting|CastToBP_InfiniteTerrainGameMode (Game|GetGameMode)))
      (Default|RemoveTile _asbp_infinite_terrain_game_mode))))

(event EventBeginPlay
  (Rendering|Material|SetMaterial (Variables|Default|GetWall) 0 "/Game/Dynamic/Terrain/MI_RedBarrier.MI_RedBarrier")
  (Class|Tile|PlaceActors "/Game/Dynamic/Terrain/Props/BP_Container.BP_Container_C" 1 5 4e+02 1.0 1.0)
  (Class|Tile|PlaceActors "/Game/Dynamic/Terrain/Props/BP_SandBagWall.BP_SandBagWall_C" 1 6 2.5e+02 1.0 1.0)
  (Class|Tile|PlaceActors "/Game/Dynamic/Terrain/Props/BP_Rock.BP_Rock_C" 1 3 1.5e+02 1.0 5.0)
  (Class|Tile|PlaceActors "/Game/Dynamic/Terrain/Props/BP_Canister.BP_Canister_C" 1 10 5e+01 1.0 3.0)
  (Class|Tile|PlaceActors "/Game/Dynamic/Terrain/Props/BP_Box.BP_Box_C" 1 1 1e+02 1.0 3.0)
  (Class|Tile|PlaceAiPawns "/Game/Dynamic/Character/Blueprints/TP_Character.TP_Character_C" 2 5 1e+02))

(fn ConstructionScript)

(fn GetAttachLocation
  (return (Transformation|GetWorldTransform (Variables|Default|GetArrow))))

(fn Unlock
  (Collision|SetCollisionEnabled (Variables|Default|GetWall) "NoCollision")
  (Rendering|Material|SetMaterial (Variables|Default|GetWall) 0 "/Game/Dynamic/Terrain/MI_SeeThrough.MI_SeeThrough"))

(fn Lock
  (Collision|SetCollisionEnabled (Variables|Default|GetWall) "QueryAndPhysics")
  (Rendering|Material|SetMaterial (Variables|Default|GetWall) 0 "/Game/Dynamic/Terrain/MI_RedBarrier.MI_RedBarrier"))