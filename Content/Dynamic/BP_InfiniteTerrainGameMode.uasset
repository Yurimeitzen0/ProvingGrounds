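; Game mode that builds endless terrain from a chain of BP_Floor tiles.
; On BeginPlay it populates a NavMesh bounds volume pool and spawns the first tile.
; SpawnTile places each new tile at the previous one's attach location and hands it the pool.
; RemoveTile skips its first call via a counter, then destroys the oldest tile on each later call.
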(event EventBeginPlay
  (bind _terrain (Variables|Default|GetTerrain))
  (Class|InfiniteTerrainGameMode|PopulateBoundsVolumePool)
  (bind _returnvalue (Game|SpawnActorfromClass "/Game/Dynamic/Terrain/BP_Floor.BP_Floor_C" (Variables|Default|GetSpawnPoint) "Undefined" 0 0))
  (Utilities|Array|Add _terrain _returnvalue)
  (bind _attachtransform (Default|GetAttachLocation (Utilities|Array|Get(acopy) _terrain)))
  (Variables|Default|SetSpawnPoint _attachtransform))

(event EventTick
  (params (DeltaSeconds :type Float%20%28single-precision%29)))

(fn ConstructionScript)

(fn SpawnTile
  (bind _terrain (Variables|Default|GetTerrain))
  (bind _returnvalue (Game|SpawnActorfromClass "/Game/Dynamic/Terrain/BP_Floor.BP_Floor_C" (Variables|Default|GetSpawnPoint) "Undefined" 0 0))
  (Class|Tile|SetPool _returnvalue (Variables|Default|GetNavMeshBoundsVolumePool))
  (Utilities|Array|Add _terrain _returnvalue)
  (bind _attachtransform (Default|GetAttachLocation (Utilities|Array|Get(acopy) _terrain (Utilities|Array|LastIndex _terrain))))
  (Variables|Default|SetSpawnPoint _attachtransform))

(fn RemoveTile
  (bind _terrain (Variables|Default|GetTerrain))
  (switch int (Variables|Default|GetCounter)
    (:0
      (Math|Integer|IncrementInt (Variables|Default|GetCounter)))
    (:1
      (if (Utilities|Array|IsValidIndex _terrain)
        (Actor|DestroyActor (Utilities|Array|Get(acopy) _terrain))
        (Utilities|Array|RemoveIndex _terrain)
        (if (>= (Variables|Default|GetCounter) 1)
          (Variables|Default|SetCounter 1))))))